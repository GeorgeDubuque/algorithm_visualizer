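; BP_GraphEdge is a graph edge actor in an algorithm visualization that animates a sphere traveling along the edge.
; The Travel event prints a debug string and reveals the sphere, but does not itself set IsTraveling or StartTime.
; While IsTraveling, Tick moves the sphere from the actor toward Arrow using a curve-eased, time-based lerp.
; On arrival it hides the sphere, clears the flag and calls DFSProcessNextState on AlgVis_GameMode to advance the depth-first search.
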(event EventBeginPlay)

(event Collision|EventActorBeginOverlap
  (params (OtherActor :type Actor%20Object%20Reference)))

(event EventTick
  (params (DeltaSeconds :type Float%20%28single-precision%29))
  (bind _returnvalue (Utilities|Time|GetTimeSeconds))
  (bind _returnvalue_2 (Transformation|GetActorLocation))
  (bind _arrow (Variables|Default|GetArrow))
  (bind _movmentcurve (Variables|Default|GetMovmentCurve))
  (bind _starttime (Variables|Default|GetStartTime))
  (bind _movement_time (Variables|Default|GetMovement%20Time))
  (bind _returnvalue_3 (Transformation|GetActorLocation _arrow))
  (bind _returnvalue_4 (- _returnvalue _starttime))
  (bind _returnvalue_5 (/ _returnvalue_4 _movement_time))
  (bind _returnvalue_6 (Class|KismetMathLibrary|GetRuntimeFloatCurveValue _movmentcurve _returnvalue_5 0.0))
  (bind _returnvalue_7 (Math|Vector|Lerp(Vector) _returnvalue_2 _returnvalue_3 _returnvalue_6))
  (if (Variables|Default|GetIsTraveling)
    (Transformation|SetWorldLocation (Variables|Default|GetSphere) _returnvalue_7 false true)
    (if (Utilities|Operators|EqualEqual _returnvalue_7 _returnvalue_3 0.0)
      (Rendering|SetVisibility (Variables|Default|GetSphere) false false)
      (Variables|Default|SetIsTraveling false)
      (bind _asalg_vis_game_mode (Utilities|Casting|CastToAlgVis_GameMode (Game|GetGameMode)))
      (Class|AlgVisGameMode|DFSProcessNextState _asalg_vis_game_mode))))

(event EventTravel
  (Development|PrintString "Travel")
  (Rendering|SetVisibility (Variables|Default|GetSphere) true false))

(fn ConstructionScript)
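; BP_GraphNodeNew is a node in a visual graph that animates when visited and passes a traversal along to its next node.
; On BeginPlay it registers itself as Owner on its mesh's animation Blueprint.
; OnVisited stores the next node and sets the ShouldGetBigger animation flag.
; OnVisitedFinished looks up the edge to that node by name in VisualEdges and calls Travel on it.
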(event Custom|OnVisitedFinished
  (bind _visualedges (Variables|Default|GetVisualEdges))
  (bind _nextnode (Variables|Default|GetNextNode))
  (bind _nodename (Variables|/Script/algorithm_visualizer.GraphNode|GetNodeName _nextnode))
  (bind (_value _returnvalue) (Utilities|Map|Find _visualedges _nodename))
  (if (Utilities|IsValid _nextnode)
    (if _returnvalue
      (Class|NodeEdge|Travel _value))))

(event EventBeginPlay
  (bind _asgraph_node_skeleton_anim_blueprint (Utilities|Casting|CastTograph_node_Skeleton_AnimBlueprint (Components|SkeletalMesh|GetAnimInstance (Variables|Default|GetStaticMesh))))
  (Variables|/Game/Meshes/graph_node_Skeleton_AnimBlueprint.graph_node_Skeleton_AnimBlueprint_C|SetOwner _asgraph_node_skeleton_anim_blueprint self))

(event Collision|EventActorBeginOverlap
  (params (OtherActor :type Actor%20Object%20Reference)))

(event EventTick
  (params (DeltaSeconds :type Float%20%28single-precision%29)))

(event EventOnVisited
  (params (NextNode :type Graph%20Node%20Object%20Reference))
  (Variables|Default|SetNextNode NextNode)
  (bind _asgraph_node_skeleton_anim_blueprint (Utilities|Casting|CastTograph_node_Skeleton_AnimBlueprint (Components|SkeletalMesh|GetAnimInstance (Variables|Default|GetStaticMesh))))
  (Variables|/Game/Meshes/graph_node_Skeleton_AnimBlueprint.graph_node_Skeleton_AnimBlueprint_C|SetShouldGetBigger _asgraph_node_skeleton_anim_blueprint true))

(fn ConstructionScript)